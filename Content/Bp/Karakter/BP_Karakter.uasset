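; Player character Blueprint handling movement, camera look, jumping, sprinting and a P-key pause menu.
; Tick derives moving and airborne states from velocity, resetting the arm and leg components when idle or posing them mid-jump.
; Limbs animate procedurally through two Timelines, normal and fast, that drive opposing pitch rotations on paired arms and legs.
; Sprint input changes max walk speed and, while moving, starts the fast Timeline and audio, stopping both on release.
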(event `self.ReceiveTick`
  (params (DeltaSeconds :type "Float (single-precision)"))
  (bind (_returnvalue_x _returnvalue_y _returnvalue_z) (`KismetMathLibrary.BreakVector` (`self.GetVelocity`)))
  (`|ExecutionSequence`
    (:`then_0`
      (if (== (`KismetMathLibrary.VSize` (`KismetMathLibrary.MakeVector` _returnvalue_x _returnvalue_y)) 0.0)
        (set `self.HareketliMi` false)
        (if (not (`self.ZıplıyorMu`))
          (`SceneComponent.K2_SetRelativeRotation` :`self` (`self.Kol1`))
          (`SceneComponent.K2_SetRelativeRotation` :`self` (`self.Bacak1`))
          (`SceneComponent.K2_SetRelativeRotation` :`self` (`self.Bacak2`))
          (`SceneComponent.K2_SetRelativeRotation` :`self` (`self.Kol2`)))
        (else
          (set `self.HareketliMi` true))))
    (:`then_1`
      (if (== _returnvalue_z 0.0)
        (set `self.ZıplıyorMu` false)
        (else
          (set `self.ZıplıyorMu` true)
          (`SceneComponent.K2_SetRelativeRotation` (`self.Kol1`) (struct :`Pitch` 20.0) false false)
          (`SceneComponent.K2_SetRelativeRotation` (`self.Bacak1`) (struct :`Pitch` 20.0) false false)
          (`SceneComponent.K2_SetRelativeRotation` (`self.Kol2`) (struct :`Pitch` -20.0) false false)
          (`SceneComponent.K2_SetRelativeRotation` (`self.Bacak2`) (struct :`Pitch` -20.0) false false))))))

(event `InputAxis|İleriGeriHareket`
  (params (AxisValue :type "Float (single-precision)"))
  (bind (_returnvalue_roll _returnvalue_pitch _returnvalue_yaw) (`KismetMathLibrary.BreakRotator` (`self.GetControlRotation`)))
  (`self.AddMovementInput` (`KismetMathLibrary.GetForwardVector` (`KismetMathLibrary.MakeRotator` 0.0 0.0 _returnvalue_yaw)) AxisValue)
  (if (`self.HareketliMi`)
    (if (`self.HızlıMı`)
      (bind (_direction `_sağ` _sol) (`Timeline|Hareket` :!via `Stop` :!label _label)
        (:`Update`
          (`|ExecutionSequence`
            (:`then_0`
              (`SceneComponent.K2_SetRelativeRotation` (`self.Kol1`) (`KismetMathLibrary.MakeRotator` 0.0 `_sağ`) false false))
            (:`then_1`
              (`SceneComponent.K2_SetRelativeRotation` (`self.Bacak1`) (`KismetMathLibrary.MakeRotator` 0.0 `_sağ`) false false))
            (:`then_2`
              (`SceneComponent.K2_SetRelativeRotation` (`self.Kol2`) (`KismetMathLibrary.MakeRotator` 0.0 _sol) false false))
            (:`then_3`
              (`SceneComponent.K2_SetRelativeRotation` (`self.Bacak2`) (`KismetMathLibrary.MakeRotator` 0.0 _sol) false false)))))
      (else
        (goto _label)))))

(event `InputAxis|SağaSolaHareket`
  (params (AxisValue :type "Float (single-precision)"))
  (bind (_returnvalue_roll _returnvalue_pitch _returnvalue_yaw) (`KismetMathLibrary.BreakRotator` (`self.GetControlRotation`)))
  (`self.AddMovementInput` (`KismetMathLibrary.GetRightVector` (`KismetMathLibrary.MakeRotator` 0.0 0.0 _returnvalue_yaw)) AxisValue))

(event `InputAxis|YukarıAşağıBakma`
  (params (AxisValue :type "Float (single-precision)"))
  (`self.AddControllerPitchInput` AxisValue))

(event `InputAxis|SağaSolaBakma`
  (params (AxisValue :type "Float (single-precision)"))
  (`self.AddControllerYawInput` AxisValue))

(event `InputAction|Zıplama`
  (params (Key :type "Key Structure"))
  (:`Pressed`
    (`self.Jump`)))

(event `InputAction|Hızlanma`
  (params (Key :type "Key Structure"))
  (bind _charactermovement (`self.CharacterMovement`))
  (:`Pressed`
    (set `CharacterMovementComponent.MaxWalkSpeed` 30000.0 _charactermovement)
    (set `self.HızlıMı` true)
    (if (`self.HareketliMi`)
      (bind _returnvalue (`AddComponent|NODE_AddAudioComponent-14`))
      (`AudioComponent.Play` _returnvalue 0.0)
      (bind (_direction `_sağ` _sol) (`Timeline|HızlıHareket` :!label _label_2)
        (:`Update`
          (`|ExecutionSequence`
            (:`then_0`
              (`SceneComponent.K2_SetRelativeRotation` (`self.Kol1`) (`KismetMathLibrary.MakeRotator` 0.0 `_sağ`) false false))
            (:`then_1`
              (`SceneComponent.K2_SetRelativeRotation` (`self.Bacak1`) (`KismetMathLibrary.MakeRotator` 0.0 `_sağ`) false false))
            (:`then_2`
              (`SceneComponent.K2_SetRelativeRotation` (`self.Kol2`) (`KismetMathLibrary.MakeRotator` 0.0 _sol) false false))
            (:`then_3`
              (`SceneComponent.K2_SetRelativeRotation` (`self.Bacak2`) (`KismetMathLibrary.MakeRotator` 0.0 _sol) false false)))))))
  (:`Released`
    (set `CharacterMovementComponent.MaxWalkSpeed` 600.0 _charactermovement)
    (set `self.HızlıMı` false)
    (`AudioComponent.Stop` _returnvalue)
    (goto _label_2 :!via `Stop`)))

(event `Key|P`
  (params (Key :type "Key Structure"))
  (bind _returnvalue (`GameplayStatics.GetPlayerController` 0))
  (:`Pressed`
    (`GameplayStatics.SetGamePaused` true)
    (bind _returnvalue_2 (`|CreateWidget` "/Game/UI/PauseMenu/WB_PauseMenu.WB_PauseMenu_C"))
    (`UserWidget.AddToViewport` _returnvalue_2 0)
    (bind _output_get (set `PlayerController.bShowMouseCursor` true _returnvalue))
    (`WidgetBlueprintLibrary.SetInputMode_UIOnlyEx` _returnvalue null "DoNotLock" _output_get)))

(fn `UserConstructionScript`)